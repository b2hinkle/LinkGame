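; Sword item for the Link game that a Link_BP character can pick up and drop, gated by a Pickupable flag.
; Pickup turns off box physics, sets it to overlap, snaps to the RightHand mesh socket and adds to the character's Swords array.
; Drop calls detach on the passed character rather than the sword, removes the sword from Swords and re-enables pickup without restoring physics or collision.
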(event Custom|Pickup
  (params (TPCharacter :type Third%20Person%20Character%20Object%20Reference))
  (bind _box (Variables|Default|GetBox))
  (if (Variables|Default|GetbPickupable)
    (bind _aslink_bp (Utilities|Casting|CastToLink_BP TPCharacter))
    (Collision|SetCollisionProfileName _box "OverlapAll" true :!class /Script/Engine.PrimitiveComponent)
    (Physics|SetSimulatePhysics _box false)
    (Transformation|AttachComponentToComponent (Variables|/Script/Engine.Character|GetMesh _aslink_bp) "RightHand" "SnapToTarget" "SnapToTarget" "KeepRelative" true)
    (Utilities|Array|Add (Variables|/Game/Blueprints/ThirdPerson/SwordCharacter.SwordCharacter_C|GetSwords _aslink_bp) 0)
    (Variables|Default|SetbPickupable false)))

(event Custom|Drop
  (params (TPCharacter :type Third%20Person%20Character%20Object%20Reference))
  (Transformation|DetachFromActor TPCharacter "KeepRelative" "KeepRelative" "KeepRelative")
  (bind _aslink_bp (Utilities|Casting|CastToLink_BP TPCharacter))
  (Utilities|Array|RemoveItem (Variables|/Game/Blueprints/ThirdPerson/SwordCharacter.SwordCharacter_C|GetSwords _aslink_bp) self)
  (Variables|Default|SetbPickupable true))

(event EventBeginPlay)

(event Collision|EventActorBeginOverlap
  (params (OtherActor :type Actor%20Object%20Reference)))

(event EventTick
  (params (DeltaSeconds :type Float%20%28single-precision%29)))

(fn ConstructionScript)